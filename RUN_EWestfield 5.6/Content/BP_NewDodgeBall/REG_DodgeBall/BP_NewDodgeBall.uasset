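; Dodgeball actor that can be thrown and takes one health point from any third-person character it hits.
; ThrowBall adds a projectile movement component at runtime, sets its velocity from the fire direction and projectile speed, then enables mesh collision.
; Hit casts to the character, lowers its health and refreshes its health widget directly.
; LaunchBall is a stub applying zero impulse, and a detach-before-throw chain is left disconnected.
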(event Custom|ThrowBall
  (params (FireDirection :type Vector) (player :type Actor%20Object%20Reference))
  (bind _returnvalue (AddComponent|AddProjectileMovementComponent))
  (Variables|/Script/Engine.MovementComponent|SetVelocity _returnvalue (* FireDirection (Variables|Default|GetProjectileSpeed)))
  (Collision|SetCollisionEnabled (Variables|Default|GetBallMesh) "QueryAndPhysics"))

(event EventBeginPlay)

(event Collision|EventActorBeginOverlap
  (params (OtherActor :type Actor%20Object%20Reference)))

(event Collision|EventHit
  (params (MyComp :type Primitive%20Component%20Object%20Reference) (Other :type Actor%20Object%20Reference) (OtherComp :type Primitive%20Component%20Object%20Reference) (bSelfMoved :type Boolean) (HitLocation :type Vector :default "0, 0, 0") (HitNormal :type Vector :default "0, 0, 0") (NormalImpulse :type Vector :default "0, 0, 0") (Hit :type Hit%20Result%20Structure%20%28by%20ref%29))
  (bind _asbp_third_person_character (Utilities|Casting|CastToBP_ThirdPersonCharacter Other))
  (bind _output_get (Variables|/Game/ThirdPerson/Blueprints/BP_ThirdPersonCharacter.BP_ThirdPersonCharacter_C|SetCurrentHealth _asbp_third_person_character (- (Variables|/Game/ThirdPerson/Blueprints/BP_ThirdPersonCharacter.BP_ThirdPersonCharacter_C|GetCurrentHealth _asbp_third_person_character) 1)))
  (Default|SetHealth (Variables|/Game/ThirdPerson/Blueprints/BP_ThirdPersonCharacter.BP_ThirdPersonCharacter_C|GetHealthWidget _asbp_third_person_character) _output_get (Variables|/Game/ThirdPerson/Blueprints/BP_ThirdPersonCharacter.BP_ThirdPersonCharacter_C|GetMaxHealth _asbp_third_person_character)))

(fn ConstructionScript)

(fn LaunchBall
  (params (Directions :type Vector))
  (Physics|AddImpulse (Variables|Default|GetBallMesh) "0, 0, 0" "None" false))